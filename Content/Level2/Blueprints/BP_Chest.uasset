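; BP_Chest is a Level 2 chest that opens only when the player character holds both the Red and Blue keys.
; OpenChest casts the player to BP_FirstPersonCharacter, checks HasKey for each color, then sets IsOpen so it cannot open again.
; A timeline then lerps the lid's relative location and roll to swing it open.
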(event Custom|OpenChest
  ;[1 1 1] Check can open chest
  (if (not (Variables|Default|GetIsOpen))
    (bind _asbp_first_person_character (Utilities|Casting|CastToBP_FirstPersonCharacter (Game|GetPlayerCharacter 0)))
    (bind _has (Default|HasKey _asbp_first_person_character "Red"))
    (if _has
      (bind _has_2 (Default|HasKey _asbp_first_person_character "Blue"))
      (if _has_2
        ;[1 1 1] Animation open chest
        (Variables|Default|SetIsOpen true)
        (bind _openchestfloat (Timeline|OpenChestTimeline Play)
          (:Update
            (Transformation|SetRelativeLocationAndRotation (Variables|Default|Getchest_chest_lid) (Math|Vector|MakeVector 0.0 (Math|Float|Lerp 0.0 3e+01 _openchestfloat) (Math|Float|Lerp 0.0 45.0 _openchestfloat)) (Math|Rotator|MakeRotator (Math|Float|Lerp 0.0 -75.0 _openchestfloat) 0.0 0.0) false false)))))))

(fn ConstructionScript)