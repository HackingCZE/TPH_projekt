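; A floor spike trap that shoots when the player steps into its trigger box and sends the player back on contact.
; After a short delay, a timeline lerps the parent component's height and plays the shoot sound once per activation.
; A flag blocks retriggering until a cooldown, started from the timeline's update, ends.
; Either spike mesh overlapping the player calls TeleportToSpikeCheck on BP_FirstPersonCharacter.
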(event OnComponentBeginOverlap(Box)
  (params (OverlappedComponent :type Primitive%20Component%20Object%20Reference) (OtherActor :type Actor%20Object%20Reference) (OtherComp :type Primitive%20Component%20Object%20Reference) (OtherBodyIndex :type Integer) (bFromSweep :type Boolean) (SweepResult :type Hit%20Result%20Structure%20%28by%20ref%29))
  ;[1 1 1] Check can go up
  (if (Actor|ActorHasTag OtherActor "Player")
    (if (Variables|Default|GetCanAgain)
      (Variables|Default|SetPlayed false)
      (Variables|Default|SetCanAgain false)
      (Utilities|FlowControl|Delay 0.6)
      ;[1 1 1] Animation and sound
      (bind _movefloat (Timeline|Timeline_0 PlayFromStart)
        (:Update
          (Transformation|SetRelativeLocation (Variables|Default|GetParent) (Math|Vector|MakeVector 0.0 0.0 (Math|Float|Lerp (Variables|Default|GetVar1) (Variables|Default|GetVar2) _movefloat)) false false)
          (if (Variables|Default|GetPlayed)
            _
            (else
              (Variables|Default|SetPlayed true)
              (Audio|PlaySound2D "/Game/Level2/Sounds/Spike_shoot.Spike_shoot" 1.0 1.0 0.0 0 0)))
          (Utilities|FlowControl|Delay 4.0)
          (Variables|Default|SetCanAgain true))))))

(event OnComponentBeginOverlap(floor_tile_big_spikes_spikes)
  (params (OverlappedComponent :type Primitive%20Component%20Object%20Reference) (OtherActor :type Actor%20Object%20Reference) (OtherComp :type Primitive%20Component%20Object%20Reference) (OtherBodyIndex :type Integer) (bFromSweep :type Boolean) (SweepResult :type Hit%20Result%20Structure%20%28by%20ref%29))
  ;[1 1 1] Check collision
  (if (Actor|ActorHasTag OtherActor "Player")
    (Development|PrintString "hit")
    (bind _asbp_first_person_character (Utilities|Casting|CastToBP_FirstPersonCharacter OtherActor))
    (Default|TeleporttoSpikeCheck _asbp_first_person_character)))

(event OnComponentBeginOverlap(floor_tile_big_spikes_spikes1)
  (params (OverlappedComponent :type Primitive%20Component%20Object%20Reference) (OtherActor :type Actor%20Object%20Reference) (OtherComp :type Primitive%20Component%20Object%20Reference) (OtherBodyIndex :type Integer) (bFromSweep :type Boolean) (SweepResult :type Hit%20Result%20Structure%20%28by%20ref%29))
  ;[1 1 1] Check collision
  (if (Actor|ActorHasTag OtherActor "Player")
    (Development|PrintString "hit")
    (bind _asbp_first_person_character (Utilities|Casting|CastToBP_FirstPersonCharacter (stale OnComponentBeginOverlap(floor_tile_big_spikes_spikes) OtherActor)))
    (Default|TeleporttoSpikeCheck _asbp_first_person_character)))

(fn ConstructionScript)