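; BP_ShootTrap is a Level 2 trap that repeatedly fires BP_Projectile actors from its own transform.
; Shoot sets a CanAgain flag and starts a latent Delay loop: short random wait, spawn, sound at the Arrow component, then a TimeToNext pause.
; StopShoot clears the flag, so the loop ends at its next check; a shot already pending still fires.
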(event Custom|Shoot
  ;[1 1 1] ShootPlate
  (Variables|Default|SetCanAgain true)
  (if (Variables|Default|GetCanAgain) :!label _label
    (Development|PrintString "shoot")
    (Utilities|FlowControl|Delay (Math|Random|RandomFloatinRange 0.0 0.3))
    (Game|SpawnActorfromClass "/Game/Level2/Blueprints/BP_Projectile.BP_Projectile_C" (Transformation|GetActorTransform) "AlwaysSpawn" "MultiplyWithRoot" 0 0)
    (Audio|PlaySoundatLocation "/Game/Level2/Sounds/Shoot_plate.Shoot_plate" (Transformation|GetWorldLocation (Variables|Default|GetArrow)) "0, 0, 0" 1.0 1.0 0.0 0 0 0 0)
    (Utilities|FlowControl|Delay (Variables|Default|GetTimeToNext))
    (goto _label)))

(event Custom|StopShoot
  ;[1 1 1] Stop loop shoting
  (Variables|Default|SetCanAgain false))

(fn ConstructionScript)