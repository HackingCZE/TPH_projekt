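; BP_Door is a door that toggles open and closed, gated by either keys or locks.
; OpenDoor requires the player's Red and Blue keys when MustHaveKeys is set; otherwise it checks Locks, tries keys on closed ones, and lets the last lock decide CanOpen.
; With no locks it opens freely.
; A FlipFlop alternates playing and reversing a timeline that lerps door yaw toward Angle, playing a sound once per trigger.
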(event Custom|OpenDoor
  (bind _door (Variables|Default|GetDoor))
  ;[1 1 1] Check open door
  (if (Variables|Default|GetMustHaveKeys)
    ;[1 1 1] Must have red and blue keys
    (bind _asbp_first_person_character (Utilities|Casting|CastToBP_FirstPersonCharacter (Game|GetPlayerCharacter 0)))
    (bind _has (Default|HasKey _asbp_first_person_character "Red"))
    (if _has
      (bind _has_2 (Default|HasKey _asbp_first_person_character "Blue"))
      (if _has_2
        ;[1 1 1] Open Door
        (Variables|Default|SetCanOpen true :!label _label)
        (if (Variables|Default|GetCanOpen) :!label _label_2
          (Variables|Default|SetPlayed false)
          (Utilities|FlowControl|FlipFlop
            (:A
              (bind _doorfloat (Timeline|OpenDoorTimeline Play)
                (:Update
                  (Transformation|SetRelativeRotation _door (Math|Rotator|MakeRotator 0.0 0.0 (Math|Float|Lerp (.yaw (Transformation|GetWorldRotation _door)) (Variables|Default|GetAngle) _doorfloat)) false false)
                  (if (not (Variables|Default|GetPlayed))
                    (Variables|Default|SetPlayed true)
                    (Audio|PlaySound2D "/Game/Level2/Sounds/open_door.open_door" 1.0 1.0 0.0 0 0)))))
            (:B
              (Timeline|OpenDoorTimeline ReverseFromEnd))))))
    (elif (> (Utilities|Array|Length (Variables|Default|GetLocks)) 0)
      (for _array_element (Variables|Default|GetLocks)
        ;[1 1 1] Check locks
        (if (Variables|/Game/Level2/Blueprints/BP_Lock.BP_Lock_C|GetIsOpen _array_element)
          (Variables|Default|SetCanOpen true)
          (else
            (Default|TryAddKey _array_element)
            (Variables|Default|SetCanOpen false))))
      (goto _label_2)
      (else
        (goto _label)))))

(fn ConstructionScript)