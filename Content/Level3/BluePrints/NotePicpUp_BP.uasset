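; NotePicpUp_BP is a readable note/book pickup that notifies BP_bookshelf actors once it has been read.
; Actor overlap enables and disables its input, where E drives a FlipFlop.
; The first press shows WBP_NotePaperWidget and hides the mesh.
; The next removes the widget, restores the mesh, sets IsPickUp and passes it to every bookshelf through IsPickUpMessage.
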(event Collision|EventActorBeginOverlap
  (params (OtherActor :type Actor%20Object%20Reference))
  ;[1 1 1] Box Collision with Book
  (Input|EnableInput (Game|GetPlayerController 0))
  (Utilities|Casting|CastToBP_FirstPersonCharacter (Game|GetPlayerCharacter 0)))

(event Collision|EventActorEndOverlap
  (params (OtherActor :type Actor%20Object%20Reference))
  ;[1 1 1] Box Collision with Book
  (Input|DisableInput 0))

(event Input|KeyboardEvents|E
  (params (Key :type Key%20Structure))
  ;[1 1 1] Pick Up the Book destroy it when it is readeing and then set variable to IsPickUp True
  (:Pressed
    (Utilities|FlowControl|FlipFlop
      (:A
        (bind _returnvalue (UserInterface|CreateWidget "/Game/Level3/Widget/WBP_NotePaperWidget.WBP_NotePaperWidget_C"))
        (UserInterface|Viewport|AddtoViewport _returnvalue 0)
        (Rendering|SetVisibility (Variables|Default|GetStaticMesh) false false))
      (:B
        (Widget|RemovefromParent _returnvalue)
        (Rendering|SetVisibility (Variables|Default|GetStaticMesh) true false)
        (Variables|Default|SetisPickUp true)
        (bind _outactors (Actor|GetAllActorsOfClass "/Game/Level3/BluePrints/BP_bookshelf.BP_bookshelf_C"))
        (Class|BookDoorOpen|IsPickUp(Message) _outactors (Variables|Default|GetisPickUp))))))

(fn ConstructionScript)