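; BP_knife is a collectible knife that the first-person character picks up with E in Level 3.
; Box overlap enables and disables the actor's own input, so the key works only within range.
; Pickup plays a sound at the knife and a scary 2D sound, destroys the actor and sets IsKnifeCollected.
; It passes that flag through an interface message to the BP_wallLanternBP found by GetActorOfClass.
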(event OnComponentBeginOverlap(Box)
  (params (OverlappedComponent :type Primitive%20Component%20Object%20Reference) (OtherActor :type Actor%20Object%20Reference) (OtherComp :type Primitive%20Component%20Object%20Reference) (OtherBodyIndex :type Integer) (bFromSweep :type Boolean) (SweepResult :type Hit%20Result%20Structure%20%28by%20ref%29))
  ;[1 1 1] Box Collision with Knige
  (Utilities|Casting|CastToBP_FirstPersonCharacter OtherActor)
  (Input|EnableInput (Game|GetPlayerController 0)))

(event OnComponentEndOverlap(Box)
  (params (OverlappedComponent :type Primitive%20Component%20Object%20Reference) (OtherActor :type Actor%20Object%20Reference) (OtherComp :type Primitive%20Component%20Object%20Reference) (OtherBodyIndex :type Integer))
  ;[1 1 1] Box Collision with Knige
  (Utilities|Casting|CastToBP_FirstPersonCharacter OtherActor)
  (Input|DisableInput (Game|GetPlayerController 0)))

(event Input|KeyboardEvents|E
  (params (Key :type Key%20Structure))
  ;[1 1 1] Pick Up Knife and Set it True as Collected
  (:Pressed
    (Audio|PlaySoundatLocation "/Engine/VREditor/Sounds/UI/Object_PickUp.Object_PickUp" (Transformation|GetActorLocation) "0, 0, 0" 1.0 1.0 0.0 0 0 0 0)
    (Actor|DestroyActor)
    (Variables|Default|SetisKnifeCollected true)
    (Audio|PlaySound2D "/Game/Level3/Audio/S_scary_104_strange_walk.S_scary_104_strange_walk" 1.0 1.0 0.0 0 0)
    (bind _returnvalue (Actor|GetActorOfClass "/Game/Level3/BluePrints/BP_wallLanternBP.BP_wallLanternBP_C"))
    (Class|BIKnifeInterface|KnifeInterface(Message) _returnvalue (Variables|Default|GetisKnifeCollected))))

(fn ConstructionScript)