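; BP_collectable is a key pickup in Level 3 that the player collects by pressing E.
; Its Box overlap with BP_FirstPersonCharacter enables input on the actor for player controller 0, and ending the overlap disables it.
; On E, it plays a pickup sound, casts the game mode to BP_FirstPersonGameMode, calls CallKeyDisp and destroys itself.
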(event OnComponentBeginOverlap(Box)
  (params (OverlappedComponent :type Primitive%20Component%20Object%20Reference) (OtherActor :type Actor%20Object%20Reference) (OtherComp :type Primitive%20Component%20Object%20Reference) (OtherBodyIndex :type Integer) (bFromSweep :type Boolean) (SweepResult :type Hit%20Result%20Structure%20%28by%20ref%29))
  ;[1 1 1] Box Collision with Key
  (Utilities|Casting|CastToBP_FirstPersonCharacter OtherActor)
  (Input|EnableInput (Game|GetPlayerController 0)))

(event OnComponentEndOverlap(Box)
  (params (OverlappedComponent :type Primitive%20Component%20Object%20Reference) (OtherActor :type Actor%20Object%20Reference) (OtherComp :type Primitive%20Component%20Object%20Reference) (OtherBodyIndex :type Integer))
  ;[1 1 1] Box Collision with Key
  (Utilities|Casting|CastToBP_FirstPersonCharacter OtherActor)
  (Input|DisableInput (Game|GetPlayerController 0)))

(event Input|KeyboardEvents|E
  (params (Key :type Key%20Structure :default "None"))
  ;[1 1 1] Pick Up Key and check if they are collected all
  (:Pressed
    (Audio|PlaySoundatLocation "/Engine/VREditor/Sounds/UI/Object_PickUp.Object_PickUp" (Transformation|GetActorLocation) "0, 0, 0" 1.0 1.0 0.0 0 0 0 0)
    (Utilities|Casting|CastToBP_FirstPersonGameMode (Game|GetGameMode))
    (Default|CallKeyDisp)
    (Actor|DestroyActor)))

(fn ConstructionScript)