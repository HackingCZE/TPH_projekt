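; BP_wall is a Level 3 wall that destroys itself once four collectables report in.
; On BeginPlay it finds every BP_collectable and binds to its KeyDisp dispatcher, counting each call in ItemsCollected through a handler named for pressure plate overlap.
; A separate CustomEvent, not called within this Blueprint, plays a collapse sound and destroys the wall when IsCollected is true; the counter path destroys it without sound.
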(event Custom|CustomEvent
  (params (isCollected :type Boolean))
  ;[1 1 1] When all Keys are Collected Destroy Wall
  (if isCollected
    (Audio|SpawnSoundatLocation "/Game/Level3/StarterContent/Audio/Collapse02.Collapse02" (Transformation|GetActorLocation) "0, 0, 0" 1.0 1.0 0.0 0 0)
    (Actor|DestroyActor)))

(event Custom|Pressure%20Plate%20Being%20Overlaped
  (bind _itemscollected (Variables|Default|GetItemsCollected))
  (Math|Integer|IncrementInt _itemscollected
    (:%20%20
      (if (== _itemscollected 4)
        (Actor|DestroyActor)))))

(event EventBeginPlay
  (bind _outactors (Actor|GetAllActorsOfClass "/Game/Level3/BluePrints/BP_collectable.BP_collectable_C"))
  (EventDispatchers|BindEventtoKeyDisp _outactors (delegate Custom|Pressure%20Plate%20Being%20Overlaped)))

(fn ConstructionScript)