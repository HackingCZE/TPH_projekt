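; Level 3 wall lantern Blueprint whose point light is hidden at BeginPlay and drives the transition to Level_4.
; Bear and knife interface events share one check that compares their collected flags for equality, intended to detect both pickups.
; A match enters a FlipFlop whose A side lights the lantern, then plays a creepy 2D sound after a delay.
; A long camera and audio fade to black simulates oxygen loss before Level_4 opens.
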(event EventBeginPlay
  ;[1 1 1] Set Visibitity of Lantern to Off when Game Starts
  (Rendering|SetVisibility (Variables|Default|GetPointLight) false false))

(event EventBearInterface
  (params (isBearCollected :type Boolean))
  ;[1 1 1] Turn On Lantern when both Bear and Knife is Collected
  (if (== isBearCollected (stale EventKnifeInterface isKnifeCollected))
    (Utilities|FlowControl|FlipFlop
      (:A
        (Rendering|SetVisibility (Variables|Default|GetPointLight) true false)
        (Utilities|FlowControl|Delay 4.0)
        ;[1 1 1] Start Playing Sound Creepy
        (Audio|PlaySound2D "/Game/Level3/Creepy-Little-Girl-Talking_-Singing_-Laughing_-Humming-_-Scary-Horror-Voice-_HD_-_FREE_.Creepy-Little-Girl-Talking_-Singing_-Laughing_-Humming-_-Scary-Horror-Voice-_HD_-_FREE_" 1.0 1.0 0.0 0 0)
        ;[1 1 1] Slowly Fading Out Screen to Black Simulation Loosing Oxygen
        (Utilities|FlowControl|Delay 0.0)
        (CameraFades|StartCameraFade :self (Game|GetPlayerCameraManager 0) :ToAlpha 1.0 :Duration 4e+01 :bShouldFadeAudio true :bHoldWhenFinished true)
        (Utilities|FlowControl|Delay 4e+01)
        (Game|OpenLevel(byName) "Level_4")))))

(event EventKnifeInterface
  (params (isKnifeCollected :type Boolean))
  ;[1 1 1] Turn On Lantern when both Bear and Knife is Collected
  (if (== (stale EventBearInterface isBearCollected) isKnifeCollected)
    (Utilities|FlowControl|FlipFlop
      (:A
        (Rendering|SetVisibility (Variables|Default|GetPointLight) true false)
        (Utilities|FlowControl|Delay 4.0)
        ;[1 1 1] Start Playing Sound Creepy
        (Audio|PlaySound2D "/Game/Level3/Creepy-Little-Girl-Talking_-Singing_-Laughing_-Humming-_-Scary-Horror-Voice-_HD_-_FREE_.Creepy-Little-Girl-Talking_-Singing_-Laughing_-Humming-_-Scary-Horror-Voice-_HD_-_FREE_" 1.0 1.0 0.0 0 0)
        ;[1 1 1] Slowly Fading Out Screen to Black Simulation Loosing Oxygen
        (Utilities|FlowControl|Delay 0.0)
        (CameraFades|StartCameraFade :self (Game|GetPlayerCameraManager 0) :ToAlpha 1.0 :Duration 4e+01 :bShouldFadeAudio true :bHoldWhenFinished true)
        (Utilities|FlowControl|Delay 4e+01)
        (Game|OpenLevel(byName) "Level_4")))))

(fn ConstructionScript)