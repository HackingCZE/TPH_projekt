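; BP_PuzzleMaster is a rotation puzzle that opens a door when three cubes reach their target rotations.
; While the first-person character is inside the trigger box, four keys each pick one preset rotation offset per cube.
; Tick, enabled per move, interpolates all cubes together, ignores new presses until done, then stores the new start rotations.
; After each move it compares cubes to CompleteRotation within a tolerance and messages the Door on success.
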(event OnComponentBeginOverlap(Box)
  (params (OverlappedComponent :type Primitive%20Component%20Object%20Reference) (OtherActor :type Actor%20Object%20Reference) (OtherComp :type Primitive%20Component%20Object%20Reference) (OtherBodyIndex :type Integer) (bFromSweep :type Boolean) (SweepResult :type Hit%20Result%20Structure%20%28by%20ref%29))
  (Utilities|Casting|CastToBP_FirstPersonCharacter OtherActor)
  (Input|EnableInput (Game|GetPlayerController 0)))

(event OnComponentEndOverlap(Box)
  (params (OverlappedComponent :type Primitive%20Component%20Object%20Reference) (OtherActor :type Actor%20Object%20Reference) (OtherComp :type Primitive%20Component%20Object%20Reference) (OtherBodyIndex :type Integer))
  (Utilities|Casting|CastToBP_FirstPersonCharacter OtherActor)
  (Input|DisableInput (Game|GetPlayerController 0)))

(event Custom|RotateStuff
  (for _array_element (Variables|Default|GetData)
    (Transformation|SetRelativeRotation (.Component (Utilities|Struct|BreakST_PuzzleData _array_element)) (Math|Rotator|CombineRotators (.StartRotation (Utilities|Struct|BreakST_PuzzleData _array_element)) (Math|Rotator|MakeRotator (* (.roll (Utilities|Array|Get(acopy) (.Rotation (Utilities|Struct|BreakST_PuzzleData _array_element)) (Variables|Default|GetRotationIndex))) (/ (Variables|Default|GetCurentTime) (Variables|Default|GetRotationTime))) (* (.pitch (Utilities|Array|Get(acopy) (.Rotation (Utilities|Struct|BreakST_PuzzleData _array_element)) (Variables|Default|GetRotationIndex))) (/ (Variables|Default|GetCurentTime) (Variables|Default|GetRotationTime))) (* (.yaw (Utilities|Array|Get(acopy) (.Rotation (Utilities|Struct|BreakST_PuzzleData _array_element)) (Variables|Default|GetRotationIndex))) (/ (Variables|Default|GetCurentTime) (Variables|Default|GetRotationTime))))) false false))
  (if (>= (Variables|Default|GetCurentTime) (Variables|Default|GetRotationTime))
    (Variables|Default|SetIsMoving false)
    (Actor|Tick|SetActorTickEnabled false)
    (Variables|Default|SetCurentTime 0.0)
    (for (_array_element_2 _array_index) (Variables|Default|GetData)
      (Transformation|SetRelativeRotation (.Component (Utilities|Struct|BreakST_PuzzleData _array_element_2)) (Math|Rotator|CombineRotators (.StartRotation (Utilities|Struct|BreakST_PuzzleData _array_element_2)) (Utilities|Array|Get(acopy) (.Rotation (Utilities|Struct|BreakST_PuzzleData _array_element_2)) (Variables|Default|GetRotationIndex))) false false)
      (Utilities|Struct|SetmembersinST_PuzzleData _array_element_2 (Math|Rotator|CombineRotators (.StartRotation (Utilities|Struct|BreakST_PuzzleData _array_element_2)) (Utilities|Array|Get(acopy) (.Rotation (Utilities|Struct|BreakST_PuzzleData _array_element_2)) (Variables|Default|GetRotationIndex))))
      (Utilities|Array|SetArrayElem :TargetArray (Variables|Default|GetData) :Index _array_index))
    (bind _succes (CallFunction|IsPuzzleCompleted))
    (if _succes
      (Class|BPInterface|DoorOpen(Message) (Variables|Default|GetDoor)))))

(event Custom|TryRotate
  (params (RotationIndex :type Integer))
  (if (not (Variables|Default|GetIsMoving))
    (Variables|Default|SetIsMoving true)
    (Variables|Default|SetRotationIndex RotationIndex)
    (Actor|Tick|SetActorTickEnabled true)))

(event EventBeginPlay
  (bind _cube1 (Variables|Default|GetCube1))
  (bind _cube2 (Variables|Default|GetCube2))
  (bind _cube3 (Variables|Default|GetCube3))
  (Utilities|Array|Add (Variables|Default|GetData) (Utilities|Struct|MakeST_PuzzleData _cube1 (Variables|/Script/Engine.SceneComponent|GetRelativeRotation _cube1) (Utilities|Array|MakeArray "10.000000,0.000000,0.000000" "25.000000,0.000000,0.000000" "-25.000000,0.000000,0.000000" "-10.000000,0.000000,0.000000")))
  (Utilities|Array|Add (Variables|Default|GetData) (Utilities|Struct|MakeST_PuzzleData _cube2 (Variables|/Script/Engine.SceneComponent|GetRelativeRotation _cube2) (Utilities|Array|MakeArray "20.000000,0.000000,0.000000" "30.000000,0.000000,0.000000" "-25.000000,0.000000,0.000000" "-30.000000,0.000000,0.000000")))
  (Utilities|Array|Add (Variables|Default|GetData) (Utilities|Struct|MakeST_PuzzleData _cube3 (Variables|/Script/Engine.SceneComponent|GetRelativeRotation _cube3) (Utilities|Array|MakeArray "40.000000,0.000000,0.000000" "35.000000,0.000000,0.000000" "-40.000000,0.000000,0.000000" "-25.000000,0.000000,0.000000"))))

(event EventTick
  (params (DeltaSeconds :type Float%20%28single-precision%29))
  (Variables|Default|SetCurentTime (+ DeltaSeconds (Variables|Default|GetCurentTime)))
  (CallFunction|RotateStuff))

(event Input|KeyboardEvents|V
  (params (Key :type Key%20Structure :default "None"))
  (:Pressed
    (CallFunction|TryRotate 3)))

(event Input|KeyboardEvents|C
  (params (Key :type Key%20Structure :default "None"))
  (:Pressed
    (CallFunction|TryRotate 2)))

(event Input|KeyboardEvents|Y
  (params (Key :type Key%20Structure :default "None"))
  (:Pressed
    (CallFunction|TryRotate)))

(event Input|KeyboardEvents|X
  (params (Key :type Key%20Structure :default "None"))
  (:Pressed
    (CallFunction|TryRotate 1)))

(fn ConstructionScript)

(fn IsPuzzleCompleted
  (for (_array_element _array_index) (Variables|Default|GetCompleteRotation)
    (if (not (Utilities|Operators|EqualEqual (Variables|/Script/Engine.SceneComponent|GetRelativeRotation (.component (Utilities|Array|Get(acopy) (Variables|Default|GetData) _array_index))) _array_element 0.5))
      (LocalVariables|SetL_Succes false)))
  (return (LocalVariables|GetL_Succes)))