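; BP_Door is a door actor in Level 4 that swings open once enough items have been collected.
; Each Collect call increments a counter, and reaching the maximum fires OpenDoor through a DoOnce gate so it triggers only once.
; OpenDoor plays a timeline that lerps the static mesh's relative yaw to rotate the door a quarter turn.
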(event Custom|Open%20Door
  (bind _open_door (Timeline|OpenDoor Play)
    (:Update
      (Transformation|SetRelativeRotation (Variables|Default|GetStaticMesh) (Math|Rotator|MakeRotator 0.0 0.0 (Math|Float|Lerp 0.0 -9e+01 _open_door)) false false))))

(event Custom|Collect
  (Math|Integer|IncrementInt (Variables|Default|GetCurrentItemCollected)
    (:%20%20
      (if (>= (Variables|Default|GetCurrentItemCollected) (Variables|Default|GetMaxItemCollectable))
        (Utilities|FlowControl|DoOnce false
          (:Completed
            (CallFunction|OpenDoor)))))))

(fn ConstructionScript)