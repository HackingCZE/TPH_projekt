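; Coll_Spike is a level trigger volume that reacts to the first player pawn entering and leaving it.
; On begin overlap it registers itself with the pawn for interaction, sends activate messages to ActivateTargets and fires OnActivated.
; On end overlap it unregisters and sends deactivate messages to DeactivateTargets.
; Both overlaps call the empty TriggerActivated hook; the empty TriggerDeactivated is never called here.
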(event OnComponentBeginOverlap(Trigger)
  (params (OverlappedComponent :type Primitive%20Component%20Object%20Reference) (OtherActor :type Actor%20Object%20Reference) (OtherComp :type Primitive%20Component%20Object%20Reference) (OtherBodyIndex :type Integer) (bFromSweep :type Boolean) (SweepResult :type Hit%20Result%20Structure%20%28by%20ref%29))
  ;[1 1 1] Trigger Activated
  (if (== OtherActor (Game|Player|GetPlayerPawn 0))
    (Class|BPIPlayer|RegisterInteraction(Message) OtherActor self)
    (CallFunction|TriggerActivated)
    (for _array_element (Variables|Default|GetActivateTargets)
      (Utilities|IsValid _array_element
        (:Is%20Valid
          (Class|BPIInteractive|Activate(Message) _array_element))))
    (Default|CallOnActivated)))

(event OnComponentEndOverlap(Trigger)
  (params (OverlappedComponent :type Primitive%20Component%20Object%20Reference) (OtherActor :type Actor%20Object%20Reference) (OtherComp :type Primitive%20Component%20Object%20Reference) (OtherBodyIndex :type Integer))
  (if (== OtherActor (Game|Player|GetPlayerPawn 0))
    (Class|BPIPlayer|UnregisterInteraction(Message) OtherActor)
    (CallFunction|TriggerActivated)
    (for _array_element (Variables|Default|GetDeactivateTargets)
      (Utilities|IsValid _array_element
        (:Is%20Valid
          (Class|BPIInteractive|Deactivate(Message) _array_element))))))

(fn ConstructionScript)

(fn TriggerActivated
  (params (Player :type Actor%20Object%20Reference)))

(fn TriggerDeactivated)