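; BP_KeyToPickup is a level key that the player picks up to gain a blue, green or red key.
; Its PickupKey event casts player 0's character to BP_FirstPersonCharacter and, based on the key's Blue, Green or Red bool, sets the matching Has-key flag on that character.
; An IsComplete flag limits the pickup to once, and the key component is destroyed afterward while the actor remains.
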(event Custom|PickupKey
  (bind _asbp_first_person_character (Utilities|Casting|CastToBP_FirstPersonCharacter (Game|GetPlayerCharacter 0)))
  (if (not (Variables|Default|GetIsComplete))
    (if (Variables|Default|GetBlue)
      (Variables|/Game/FirstPerson/Blueprints/BP_FirstPersonCharacter.BP_FirstPersonCharacter_C|SetHasBlueKey _asbp_first_person_character true)
      (Variables|Default|SetIsComplete true :!label _label)
      (Components|DestroyComponent (Variables|Default|Getkey_key))
      (elif (Variables|Default|GetGreen)
        (Variables|/Game/FirstPerson/Blueprints/BP_FirstPersonCharacter.BP_FirstPersonCharacter_C|SetHasGreenKey _asbp_first_person_character true)
        (goto _label)
        (elif (Variables|Default|GetRed)
          (Variables|/Game/FirstPerson/Blueprints/BP_FirstPersonCharacter.BP_FirstPersonCharacter_C|SetHasRedKey _asbp_first_person_character true)
          (goto _label))))))

(fn ConstructionScript)