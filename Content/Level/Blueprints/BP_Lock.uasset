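; BP_Lock is a colored padlock that opens when the first-person player character holds the key of the matching Color.
; BeginPlay applies one shared material to the key and both lock parts.
; TryAddKey checks the character's HasKey, then uses timelines to slide the key in and turn it.
; Near full turn it plays the unlock sound, pops LockUp open and sets IsOpen; without a key it briefly shows a text hint.
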(event Custom|TryAddKey
  (bind _key (Variables|Default|GetKey))
  (bind _lockup (Variables|Default|GetLockUp))
  (bind _asbp_first_person_character (Utilities|Casting|CastToBP_FirstPersonCharacter (Game|GetPlayerCharacter 0)))
  (bind _has (Default|HasKey _asbp_first_person_character (Variables|Default|GetColor)))
  (if _has
    (if (not (Variables|Default|GetOpening))
      (Variables|Default|SetOpening true)
      (Rendering|SetVisibility (Variables|Default|GetKey) true false)
      (Utilities|FlowControl|Delay 1.0)
      (bind _movey (Timeline|AddKeyTimeline Play)
        (:Update
          (Transformation|SetRelativeLocation (Variables|Default|GetKey) (Math|Vector|MakeVector 0.0 (Math|Float|Lerp 7e+01 4e+01 _movey) 0.0) false false)
          (Utilities|FlowControl|Delay 1.0)
          (bind _movey_2 (Timeline|Timeline Play)
            (:Update
              (Transformation|SetRelativeRotation _key (Math|Rotator|MakeRotator (Math|Float|Lerp 0.0 9e+01 _movey_2) 0.0 -9e+01) false false)
              (if (>= (.Roll (Math|Rotator|BreakRotator (Transformation|GetWorldRotation _key))) 85.0)
                (if (Variables|Default|GetPlayed)
                  _
                  (else
                    (Variables|Default|SetPlayed true)
                    (Audio|PlaySound2D "/Game/Level/Sounds/unlock_door.unlock_door" 1.0 1.0 0.0 0 0)))
                (Transformation|SetRelativeLocation _lockup "-10.000000,0.000000,-9.000000" false false)
                (Transformation|SetRelativeRotation _lockup (Math|Rotator|MakeRotator 0.0 -2e+01 0.0) false false)
                (Variables|Default|SetIsOpen true)))))))
    (else
      (Development|PrintString "no key")
      (Rendering|SetVisibility (Variables|Default|GetTextRender) true false)
      (Utilities|FlowControl|Delay 3.0)
      (Rendering|SetVisibility (Variables|Default|GetTextRender) false false))))

(event EventBeginPlay
  (CallFunction|SetMaterials))

(fn ConstructionScript)

(fn SetMaterials
  (bind _material (Variables|Default|GetMaterial))
  (Rendering|Material|SetMaterial (Variables|Default|GetKey) 0 _material)
  (Rendering|Material|SetMaterial (Variables|Default|GetLockDown) 1 _material)
  (Rendering|Material|SetMaterial (Variables|Default|GetLockUp) 0 _material))