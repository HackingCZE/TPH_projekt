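; BP_Boulder is a boulder actor that starts simulating physics when the player's first-person character enters its collision sphere.
; That overlap also spawns two 2D sounds, the boulder audio and the hard-work audio, and stores both audio components.
; When any actor's overlap with the boulder ends, both stored components have their active state toggled, with no check on which actor left.
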(event OnComponentBeginOverlap(SphereCollision)
  (params (OverlappedComponent :type Primitive%20Component%20Object%20Reference) (OtherActor :type Actor%20Object%20Reference) (OtherComp :type Primitive%20Component%20Object%20Reference) (OtherBodyIndex :type Integer) (bFromSweep :type Boolean) (SweepResult :type Hit%20Result%20Structure%20%28by%20ref%29))
  ;[1 1 1] Sounds
  (Utilities|Casting|CastToBP_FirstPersonCharacter OtherActor)
  (Physics|SetSimulatePhysics (Variables|Default|GetBoulder) true)
  (Utilities|FlowControl|Sequence
    (:then_0
      (bind _returnvalue (Audio|SpawnSound2D "/Game/Level1/Audio/S_Boulder_Audio.S_Boulder_Audio" 1.0 1.0 0.0 0))
      (Variables|Default|SetRockAudioComponent _returnvalue))
    (:then_1
      (bind _returnvalue_2 (Audio|SpawnSound2D "/Game/Level1/Audio/S_HardWork_Audio.S_HardWork_Audio" 1.0 1.0 0.0 0))
      (Variables|Default|SetWorkAudionComponent _returnvalue_2))))

(event Collision|EventActorEndOverlap
  (params (OtherActor :type Actor%20Object%20Reference))
  ;[1 1 1] Sounds
  (Utilities|FlowControl|Sequence
    (:then_0
      (Components|Activation|ToggleActive (Variables|Default|GetRockAudioComponent)))
    (:then_1
      (Components|Activation|ToggleActive (Variables|Default|GetWorkAudionComponent)))))

(fn ConstructionScript)