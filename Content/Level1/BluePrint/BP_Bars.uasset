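; Barred gate in Level1 that rises when the player's crank event fires.
; BeginPlay binds CrankEvent to the first-person character's crank dispatcher, and the Box's begin overlap stores the overlapped component (the Box itself).
; If that reference is valid, a delayed loop lifts it in small Z steps while toggling a 2D gate sound at start and end.
; Finish blocks replays, but is set only when the loop completes.
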(event OnComponentBeginOverlap(Box)
  (params (OverlappedComponent :type Primitive%20Component%20Object%20Reference) (OtherActor :type Actor%20Object%20Reference) (OtherComp :type Primitive%20Component%20Object%20Reference) (OtherBodyIndex :type Integer) (bFromSweep :type Boolean) (SweepResult :type Hit%20Result%20Structure%20%28by%20ref%29))
  ;[1 1 1] Open The Gate
  (Variables|Default|SetOverlapped%20Component OverlappedComponent))

(event Custom|CrankEvent
  ;[1 1 1] Init Disp
  ;[1 1 1] Open The Gate
  (Utilities|IsValid (Variables|Default|GetOverlapped%20Component)
    (:Is%20Valid
      (if (not (Variables|Default|GetFinish))
        (bind _returnvalue (Audio|CreateSound2D "/Game/Level1/Audio/S_Gate_Audio.S_Gate_Audio" 1.0 1.0 0.0 0))
        (Variables|Default|SetSound _returnvalue)
        (Components|Activation|ToggleActive (Variables|Default|GetSound))
        (Utilities|ForLoopDelayed 0 150 0.033
          (:Loop%20Body
            (Transformation|AddWorldOffset (Variables|Default|GetOverlapped%20Component) "0.000000,0.000000,2.000000" false false))
          (:Completed
            (Components|Activation|ToggleActive (Variables|Default|GetSound))
            (Variables|Default|SetFinish true)))))))

(event EventBeginPlay
  ;[1 1 1] Init Disp
  (bind _asbp_first_person_character (Utilities|Casting|CastToBP_FirstPersonCharacter (Game|GetPlayerCharacter 0)))
  (EventDispatchers|BindEventtoCrankDisp _asbp_first_person_character (delegate Custom|CrankEvent)))

(fn ConstructionScript)