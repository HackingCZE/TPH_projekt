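; Level 1 barricade wall that topples open once pressure plates report two boulder events, shifting the soundscape from cave to storm.
; BeginPlay starts cave audio and binds to every BP_Pressure_Plate's boulder event, which increments a counter.
; At two, a delayed while loop rolls the wall with a growing step, faking accelerating fall toward 80 degrees.
; Completion swaps falling audio for an impact, stops cave audio, then starts storm audio after a delay.
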(event Custom|Pressure%20Plate%20Being%20Overlaped
  (bind _bouldercount (Variables|Default|GetBoulderCount))
  ;[1 1 1] Comment
  (Math|Integer|IncrementInt _bouldercount
    (:%20%20
      (if (== _bouldercount 2)
        (bind _returnvalue (Audio|CreateSound2D "/Game/Level1/Audio/S_Falling_Stones.S_Falling_Stones" 1.0 1.0 0.0 0))
        (bind _output_get (Variables|Default|SetSoundOpening _returnvalue))
        (Components|Activation|ToggleActive _output_get)
        (Variables|Default|SetStep 0.05)
        (Utilities|WhileLoopDelayed (< (+ (.roll (Transformation|GetActorRotation)) (Variables|Default|GetStep)) 8e+01) 0.033
          (:Loop%20Body
            (Transformation|AddActorLocalRotation (Math|Rotator|MakeRotator (Variables|Default|GetStep) 0.0 0.0) false false)
            (Variables|Default|SetStep (+ (Variables|Default|GetStep) 0.05)))
          (:Completed
            (Components|Activation|ToggleActive (Variables|Default|GetSoundOpening))
            ;[1 1 1] Change sound
            (bind _returnvalue_2 (Audio|CreateSound2D "/Game/Level1/Audio/S_Falling_Impact_Audio.S_Falling_Impact_Audio" 1.0 1.0 0.0 0))
            (bind _output_get_2 (Variables|Default|SetSoundImpact _returnvalue_2))
            (Components|Activation|ToggleActive _output_get_2)
            (Components|Activation|ToggleActive (Variables|Default|GetSoundCave))
            (Utilities|FlowControl|Delay 5.0)
            (bind _returnvalue_3 (Audio|CreateSound2D "/Game/Level1/Audio/S_Storm_Audio.S_Storm_Audio" 1.0 1.0 0.0 0))
            (bind _output_get_3 (Variables|Default|SetSounStorm _returnvalue_3))
            (Components|Activation|ToggleActive _output_get_3)))))))

(event EventBeginPlay
  ;[1 1 1] Init
  (bind _outactors (Actor|GetAllActorsOfClass "/Game/Level1/BluePrint/BP_Pressure_Plate.BP_Pressure_Plate_C"))
  (EventDispatchers|BindEventtoBoulderDisp _outactors (delegate Custom|Pressure%20Plate%20Being%20Overlaped))
  (bind _returnvalue (Audio|CreateSound2D "/Game/Level1/Audio/S_Cave_Audio.S_Cave_Audio" 1.0 1.0 0.0 0))
  (bind _output_get (Variables|Default|SetSoundCave _returnvalue))
  (Components|Activation|ToggleActive _output_get)
  (Variables|Default|SetBoulderCount 0))

(fn ConstructionScript)