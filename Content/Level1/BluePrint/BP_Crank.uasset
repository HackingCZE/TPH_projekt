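; BP_Crank is a Level 1 crank that spins when the player character's crank dispatcher fires.
; On BeginPlay it binds CrankEvent to that dispatcher on BP_FirstPersonCharacter.
; Until Finish is set, the event finds cranks overlapping the player and rotates them incrementally through a delayed for-loop.
; When the loop completes, it sets Finish and removes the Interact widget.
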(event Custom|CrankEvent
  ;[1 1 1] Init Disp
  ;[1 1 1] Sprin the Crank
  (if (not (Variables|Default|GetFinish))
    (for _array_element (Collision|GetOverlappingActors (Game|GetPlayerCharacter 0) "BP_Crank_C" :!class /Script/Engine.Actor)
      (Variables|Default|SetArray%20Element _array_element)
      (Utilities|ForLoopDelayed 0 150 0.033
        (:Loop%20Body
          (Transformation|AddActorLocalRotation (Variables|Default|GetArray%20Element) "0.000000,0.000000,10.000000" false false))
        (:Completed
          (Variables|Default|SetFinish true)
          (Widget|RemovefromParent (Variables|Default|GetInteract)))))))

(event EventBeginPlay
  ;[1 1 1] Init Disp
  (bind _asbp_first_person_character (Utilities|Casting|CastToBP_FirstPersonCharacter (Game|GetPlayerCharacter 0)))
  (EventDispatchers|BindEventtoCrankDisp _asbp_first_person_character (delegate Custom|CrankEvent)))

(fn ConstructionScript)