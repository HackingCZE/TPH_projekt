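; Level 1 block Actor that moves continuously along the world Y axis.
; BeginPlay starts an endless delayed loop that offsets the Actor by Step at a fixed short interval, rather than using Tick.
; Overlapping any Actor other than the player character passes Step through a single unary operation, presumably a negation that reverses travel, under the section labelled Rotate.
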(event Collision|EventActorBeginOverlap
  (params (OtherActor :type Actor%20Object%20Reference))
  ;[1 1 1] Rotate
  (if (!= OtherActor (Game|GetPlayerCharacter 0))
    (bind _result (Math|Float|NegateFloat (Variables|Default|GetStep))
      (:%20%20
        (Variables|Default|SetStep _result)))))

(event EventBeginPlay
  ;[1 1 1] Move
  (Variables|Default|SetStep 1e+01)
  (Utilities|WhileLoopDelayed true 0.033
    (:Loop%20Body
      (Transformation|AddActorWorldOffset (Math|Vector|MakeVector 0.0 (Variables|Default|GetStep) 0.0)))))

(fn ConstructionScript)